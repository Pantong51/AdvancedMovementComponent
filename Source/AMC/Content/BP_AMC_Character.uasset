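; BP_AMC_Character is a player character Blueprint that maps input to walking, looking, sprinting and jetpacking.
; Movement axes feed AddMovementInput along the actor's forward and right vectors, while look axes are scaled by turn rates and frame delta time.
; Jetpack and Sprint actions call start and stop functions on press and release, with that logic defined outside this graph.
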(event `InputAxis|MoveForward`
  (params (AxisValue :type "Float (single-precision)"))
  (`self.AddMovementInput` (`self.GetActorForwardVector`) AxisValue))

(event `InputAction|Jetpack`
  (params (Key :type "Key Structure"))
  (:`Pressed`
    (`self.StartJetpacking`))
  (:`Released`
    (`self.StopJetpacking`)))

(event `InputAxis|MoveRight`
  (params (AxisValue :type "Float (single-precision)"))
  (`self.AddMovementInput` (`self.GetActorRightVector`) AxisValue))

(event `InputAction|Sprint`
  (params (Key :type "Key Structure"))
  (:`Pressed`
    (`self.StartSprinting`))
  (:`Released`
    (`self.StopSprinting`)))

(event `InputAxis|Turn`
  (params (AxisValue :type "Float (single-precision)"))
  (`self.AddControllerYawInput` (* AxisValue (`self.BaseTurnRate`) (`GameplayStatics.GetWorldDeltaSeconds`))))

(event `InputAxis|LookUp`
  (params (AxisValue :type "Float (single-precision)"))
  (`self.AddControllerPitchInput` (* AxisValue (`self.BaseLookUpRate`) (`GameplayStatics.GetWorldDeltaSeconds`))))

(fn `UserConstructionScript`)